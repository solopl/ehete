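; BP_Key_MufakAnahtari is the kitchen door key pickup for the first-person character.
; An outer sphere shows a WBP_Key widget label with the key's name; an inner sphere adds the (F) hint and enables actor input.
; Leaving the inner sphere disables input and restores the plain label, while leaving the outer sphere hides it.
; Pressing F sets HasMutfakAnahtari on the character and destroys the key.
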(event `Key|F`
  (params (Key :type "Key Structure"))
  (:`Pressed`
    (bind _asbp_first_person_character (cast `/Game/FirstPerson/Blueprints/BP_FirstPersonCharacter` (`GameplayStatics.GetPlayerCharacter` 0)))
    (set `/Game/FirstPerson/Blueprints/BP_FirstPersonCharacter.bHasMutfakAnahtari` true _asbp_first_person_character)
    (`self.K2_DestroyActor`)))

(event `self.Sphere_outer.OnComponentBeginOverlap`
  (params (OverlappedComponent :type "PrimitiveComponent Object Reference") (OtherActor :type "Actor Object Reference") (OtherComp :type "PrimitiveComponent Object Reference") (OtherBodyIndex :type Integer) (bFromSweep :type Boolean) (SweepResult :type "HitResult Structure (by ref)"))
  (bind _ui_kapiyazisi (`self.UI_KapiYazisi`))
  (cast `/Game/FirstPerson/Blueprints/BP_FirstPersonCharacter` OtherActor)
  (`SceneComponent.SetVisibility` _ui_kapiyazisi true false)
  (bind _aswbp_key (cast `/Game/Doors/WBP_Key` (`WidgetComponent.GetUserWidgetObject` _ui_kapiyazisi)))
  (set `TextBlock.Text` "Mutfak Kapısı Anahtarı" (`/Game/Doors/WBP_Key.AnahtarMetni` _aswbp_key)))

(event `self.Sphere_outer.OnComponentEndOverlap`
  (params (OverlappedComponent :type "PrimitiveComponent Object Reference") (OtherActor :type "Actor Object Reference") (OtherComp :type "PrimitiveComponent Object Reference") (OtherBodyIndex :type Integer))
  (cast `/Game/FirstPerson/Blueprints/BP_FirstPersonCharacter` OtherActor)
  (`SceneComponent.SetVisibility` (`self.UI_KapiYazisi`) false false))

(event `self.Sphere_inner.OnComponentBeginOverlap`
  (params (OverlappedComponent :type "PrimitiveComponent Object Reference") (OtherActor :type "Actor Object Reference") (OtherComp :type "PrimitiveComponent Object Reference") (OtherBodyIndex :type Integer) (bFromSweep :type Boolean) (SweepResult :type "HitResult Structure (by ref)"))
  (bind _ui_kapiyazisi (`self.UI_KapiYazisi`))
  (cast `/Game/FirstPerson/Blueprints/BP_FirstPersonCharacter` OtherActor)
  (`SceneComponent.SetVisibility` _ui_kapiyazisi true false)
  (bind _aswbp_key (cast `/Game/Doors/WBP_Key` (`WidgetComponent.GetUserWidgetObject` _ui_kapiyazisi)))
  (set `TextBlock.Text` "Mutfak Kapısı Anahtarı \\n (F)" (`/Game/Doors/WBP_Key.AnahtarMetni` _aswbp_key))
  (`self.EnableInput` (`GameplayStatics.GetPlayerController` 0)))

(event `self.Sphere_inner.OnComponentEndOverlap`
  (params (OverlappedComponent :type "PrimitiveComponent Object Reference") (OtherActor :type "Actor Object Reference") (OtherComp :type "PrimitiveComponent Object Reference") (OtherBodyIndex :type Integer))
  (bind _ui_kapiyazisi (`self.UI_KapiYazisi`))
  (cast `/Game/FirstPerson/Blueprints/BP_FirstPersonCharacter` OtherActor)
  (`SceneComponent.SetVisibility` _ui_kapiyazisi true false)
  (bind _aswbp_key (cast `/Game/Doors/WBP_Key` (`WidgetComponent.GetUserWidgetObject` _ui_kapiyazisi)))
  (set `TextBlock.Text` "Mutfak Kapısı Anahtarı" (`/Game/Doors/WBP_Key.AnahtarMetni` _aswbp_key))
  (`self.DisableInput` (`GameplayStatics.GetPlayerController` 0)))

(fn `UserConstructionScript`)