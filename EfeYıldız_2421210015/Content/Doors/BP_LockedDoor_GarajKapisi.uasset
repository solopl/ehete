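; Locked garage door that the first-person character can open and close with F while holding the garage key.
; An outer sphere shows a world widget with the door name and hides it on exit.
; An inner sphere changes that text to report whether the key is held and enables input only with the key, disabling it on exit.
; F alternates a timeline forward and in reverse to rotate the door.
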(event `Key|F`
  (params (Key :type "Key Structure"))
  (:`Pressed`
    (`/Engine/EditorBlueprintResources/StandardMacros.FlipFlop`
      (:`A`
        (bind (_direction _newtrack_0) (`Timeline|KapiAnimasyonu` :!label _label)
          (:`Update`
            (`SceneComponent.K2_SetRelativeRotation` (`self.Door`) (`KismetMathLibrary.RLerp` (struct) (struct :`Yaw` 90.0) _newtrack_0) false false))))
      (:`B`
        (goto _label :!via `Reverse`)))))

(event `self.Sphere_inner.OnComponentBeginOverlap`
  (params (OverlappedComponent :type "PrimitiveComponent Object Reference") (OtherActor :type "Actor Object Reference") (OtherComp :type "PrimitiveComponent Object Reference") (OtherBodyIndex :type Integer) (bFromSweep :type Boolean) (SweepResult :type "HitResult Structure (by ref)"))
  (bind _ui_kapiyazisi (`self.UI_KapiYazisi`))
  (bind _ui_kapiyazisi_2 (`self.UI_KapiYazisi`))
  (bind _asbp_first_person_character (cast `/Game/FirstPerson/Blueprints/BP_FirstPersonCharacter` OtherActor))
  (if (`/Game/FirstPerson/Blueprints/BP_FirstPersonCharacter.bHasGarajAnahtari` _asbp_first_person_character)
    (`SceneComponent.SetVisibility` _ui_kapiyazisi_2 true false)
    (bind _aswbp_locked_door (cast `/Game/Doors/WBP_LockedDoor` (`WidgetComponent.GetUserWidgetObject` _ui_kapiyazisi_2)))
    (set `TextBlock.Text` "Garaj Kapısı \\n Anahtar var (F)" (`/Game/Doors/WBP_LockedDoor.KapiMetni` _aswbp_locked_door))
    (`self.EnableInput` (`GameplayStatics.GetPlayerController` 0))
    (else
      (`SceneComponent.SetVisibility` _ui_kapiyazisi true false)
      (bind _aswbp_locked_door_2 (cast `/Game/Doors/WBP_LockedDoor` (`WidgetComponent.GetUserWidgetObject` _ui_kapiyazisi)))
      (set `TextBlock.Text` "Garaj Kapısı \\n Anahtar yok" (`/Game/Doors/WBP_LockedDoor.KapiMetni` _aswbp_locked_door_2)))))

(event `self.Sphere_inner.OnComponentEndOverlap`
  (params (OverlappedComponent :type "PrimitiveComponent Object Reference") (OtherActor :type "Actor Object Reference") (OtherComp :type "PrimitiveComponent Object Reference") (OtherBodyIndex :type Integer))
  (bind _ui_kapiyazisi (`self.UI_KapiYazisi`))
  (cast `/Game/FirstPerson/Blueprints/BP_FirstPersonCharacter` OtherActor)
  (`SceneComponent.SetVisibility` _ui_kapiyazisi true false)
  (bind _aswbp_locked_door (cast `/Game/Doors/WBP_LockedDoor` (`WidgetComponent.GetUserWidgetObject` _ui_kapiyazisi)))
  (set `TextBlock.Text` "Garaj Kapısı" (`/Game/Doors/WBP_LockedDoor.KapiMetni` _aswbp_locked_door))
  (`self.DisableInput` (`GameplayStatics.GetPlayerController` 0)))

(event `self.Sphere_outer.OnComponentBeginOverlap`
  (params (OverlappedComponent :type "PrimitiveComponent Object Reference") (OtherActor :type "Actor Object Reference") (OtherComp :type "PrimitiveComponent Object Reference") (OtherBodyIndex :type Integer) (bFromSweep :type Boolean) (SweepResult :type "HitResult Structure (by ref)"))
  (bind _ui_kapiyazisi (`self.UI_KapiYazisi`))
  (cast `/Game/FirstPerson/Blueprints/BP_FirstPersonCharacter` OtherActor)
  (`SceneComponent.SetVisibility` _ui_kapiyazisi true false)
  (bind _aswbp_locked_door (cast `/Game/Doors/WBP_LockedDoor` (`WidgetComponent.GetUserWidgetObject` _ui_kapiyazisi)))
  (set `TextBlock.Text` "Garaj Kapısı" (`/Game/Doors/WBP_LockedDoor.KapiMetni` _aswbp_locked_door)))

(event `self.Sphere_outer.OnComponentEndOverlap`
  (params (OverlappedComponent :type "PrimitiveComponent Object Reference") (OtherActor :type "Actor Object Reference") (OtherComp :type "PrimitiveComponent Object Reference") (OtherBodyIndex :type Integer))
  (cast `/Game/FirstPerson/Blueprints/BP_FirstPersonCharacter` OtherActor)
  (`SceneComponent.SetVisibility` (`self.UI_KapiYazisi`) false false))

(fn `UserConstructionScript`)