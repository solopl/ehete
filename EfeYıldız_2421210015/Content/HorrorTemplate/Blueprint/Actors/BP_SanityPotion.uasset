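; BP_SanityPotion is a sanity potion pickup for the horror character.
; Its Trigger overlap events enable the actor's input while BP_HorrorCharacter is inside and disable it on exit.
; Pressing E casts the overlap's OtherActor, sets HasPotion on the character and shows its Potion component.
; The pickup then loses its own Potion and Interact components, while the actor itself is not destroyed.
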(event `Key|E`
  (params (Key :type "Key Structure"))
  (:`Pressed`
    (bind _asbp_horror_character (cast `/Game/HorrorTemplate/Blueprint/BP_HorrorCharacter` (stale `self.Trigger.OnComponentBeginOverlap` OtherActor)))
    (set `/Game/HorrorTemplate/Blueprint/BP_HorrorCharacter.HasPotion?` true _asbp_horror_character)
    (`ActorComponent.K2_DestroyComponent` (`self.Potion`))
    (`ActorComponent.K2_DestroyComponent` (`self.Interact`))
    (`SceneComponent.SetVisibility` (`/Game/HorrorTemplate/Blueprint/BP_HorrorCharacter.Potion` _asbp_horror_character) true false)))

(event `self.Trigger.OnComponentBeginOverlap`
  (params (OverlappedComponent :type "PrimitiveComponent Object Reference") (OtherActor :type "Actor Object Reference") (OtherComp :type "PrimitiveComponent Object Reference") (OtherBodyIndex :type Integer) (bFromSweep :type Boolean) (SweepResult :type "HitResult Structure (by ref)"))
  (cast `/Game/HorrorTemplate/Blueprint/BP_HorrorCharacter` OtherActor)
  (`self.EnableInput` (`GameplayStatics.GetPlayerController` 0)))

(event `self.Trigger.OnComponentEndOverlap`
  (params (OverlappedComponent :type "PrimitiveComponent Object Reference") (OtherActor :type "Actor Object Reference") (OtherComp :type "PrimitiveComponent Object Reference") (OtherBodyIndex :type Integer))
  (cast `/Game/HorrorTemplate/Blueprint/BP_HorrorCharacter` OtherActor)
  (`self.DisableInput` (`GameplayStatics.GetPlayerController` 0)))

(fn `UserConstructionScript`)